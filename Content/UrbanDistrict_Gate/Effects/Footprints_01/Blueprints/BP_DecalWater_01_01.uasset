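; Water decal actor, apparently for footprint effects, that animates its decal's scale after a delay.
; On BeginPlay it zeroes the decal scale and waits, then optionally spawns a particle emitter at the decal location.
; A DecalSize timeline then drives the decal's world scale.
; With particles enabled, the timeline plays only if the particle asset is valid.
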(event `self.ReceiveBeginPlay`
  (bind _particle (`self.Particle`))
  (`SceneComponent.SetWorldScale3D` (`self.Decal`) (0.0 0.0 0.0))
  (`KismetSystemLibrary.Delay` (`self.Delay`))
  (if (`self.UseParticle`)
    (`/Engine/EditorBlueprintResources/StandardMacros.IsValid` _particle
      (:`Is Valid`
        (`GameplayStatics.SpawnEmitterAtLocation` _particle (`SceneComponent.K2_GetComponentLocation` (`self.Decal`)))
        (bind (_direction _decalsize) (`Timeline|DecalSize` :!label _label)
          (:`Update`
            (`SceneComponent.SetWorldScale3D` (`self.Decal`) (`KismetMathLibrary.Conv_DoubleToVector` _decalsize))))))
    (else
      (goto _label))))

(fn `UserConstructionScript`)